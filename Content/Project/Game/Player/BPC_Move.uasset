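; BPC_Move is an actor component that drives the Car_2_0 car along world X with lateral steering on Y.
; Each tick it moves the owner, ramping forward speed and steering speed up or down from the forward and down input flags, clamped between a minimum and maximum.
; Left and right flags set the sideways step, which is not scaled by delta time, and yaw the Car component slightly toward the turn.
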(event `self.ReceiveBeginPlay`
  (bind _output_get (set `self.Owner` (`self.GetOwner`)))
  (bind _ascar_2_0 (cast `/Game/Project/Game/Player2_0/Car_2_0` _output_get))
  (set `self.Car` (`/Game/Project/Game/Player2_0/Car_2_0.Car` _ascar_2_0)))

(event `self.ReceiveTick`
  (params (DeltaSeconds :type "Float (single-precision)"))
  (bind _deltaspeed (`self.Deltaspeed`))
  (bind _owner (`self.Owner`))
  (bind _car (`self.Car`))
  (bind _leftrightspeed (`self.leftRightSpeed`))
  (bind _movedown (`self.MoveDown`))
  (bind _moveforward (`self.MoveForward`))
  (bind _deltaspeed_2 (`self.Deltaspeed`))
  (bind (_returnvalue_x _returnvalue_y _returnvalue_z) (`KismetMathLibrary.BreakVector` (`Actor.K2_GetActorLocation` _owner)))
  (`|ExecutionSequence`
    (:`then_0`
      (`Actor.K2_SetActorLocation` _owner (`KismetMathLibrary.MakeVector` (+ (* DeltaSeconds (`self.Speed`)) _returnvalue_x) (+ _returnvalue_y (`self.LeftRighr`)) _returnvalue_z) false false)
      (if (or (and _moveforward _movedown) (not (or _moveforward _movedown)))
        _
        (elif (`self.MoveForward`)
          (if (>= (`self.Speed`) (`self.MaxSpeed`))
            (set `self.Speed` (`self.MaxSpeed`))
            (set `self.leftRightSpeed` (`self.leftRightSpeedMax`))
            (else
              (set `self.Speed` (+ (`self.Speed`) _deltaspeed_2))
              (set `self.leftRightSpeed` (+ (`self.leftRightSpeed`) (/ _deltaspeed_2 400.0)))))
          (elif (<= (`self.Speed`) 1.0)
            (set `self.Speed` 1.0)
            (set `self.leftRightSpeed` 1.0)
            (else
              (set `self.Speed` (- (`self.Speed`) _deltaspeed))
              (set `self.leftRightSpeed` (- (`self.leftRightSpeed`) (/ _deltaspeed 400.0))))))))
    (:`then_1`
      (if (or (and (`self.LeftMove`) (`self.RightMove`)) (not (or (`self.LeftMove`) (`self.RightMove`))))
        (set `self.LeftRighr` 0.0)
        (`SceneComponent.K2_SetRelativeRotation` (`self.Car`) (`KismetMathLibrary.MakeRotator` 90.0 0.0 180.0) false false)
        (elif (`self.LeftMove`)
          (set `self.LeftRighr` (* _leftrightspeed -1.0))
          (`SceneComponent.K2_SetRelativeRotation` _car (`KismetMathLibrary.MakeRotator` 90.0 0.0 170.0) false false)
          (else
            (set `self.LeftRighr` _leftrightspeed)
            (`SceneComponent.K2_SetRelativeRotation` _car (`KismetMathLibrary.MakeRotator` 90.0 0.0 190.0) false false)))))))